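; Player controller with an orbit camera that can take direct control of a selected character or wheeled vehicle.
; The server spawns and possesses BP_PlayerCamera at a PlayerStart; mouse input sets rotation and zoom, smoothed in Tick outside dedicated servers.
; X toggles server-side possession, saving and restoring the pawn's AI controller while keeping the camera view.
; During control, move axes drive the pawn and a timer aims it at the cursor when stationary.
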(event `InputAction|MouseClickRight`
  (params (Key :type "Key Structure"))
  (bind _camerapawn (`self.CameraPawn`))
  (:`Pressed`
    (set `/Game/Blueprint/Player/BP_PlayerCamera.IsRotatior` true _camerapawn))
  (:`Released`
    (set `/Game/Blueprint/Player/BP_PlayerCamera.IsRotatior` false _camerapawn)))

(event `SendServer_DisableInputPawn`
  (`/Engine/EditorBlueprintResources/StandardMacros.IsValid` (`self.AICharacter`)
    (:`Is Valid`
      (`self.Possess` (`self.AICharacter`) (`self.PawnInput`))
      (`self.Possess` (`self.CameraPawn`))
      (set `self.PawnInput` null)
      (set `self.AICharacter` null)
      (set `self.InputCharacter` false)
      (`self.SetViewTargetWithBlend` (`self.CameraPawn`)))))

(event `Key|MiddleMouseButton`
  (params (Key :type "Key Structure"))
  (bind _camerapawn (`self.CameraPawn`))
  (:`Pressed`
    (set `/Game/Blueprint/Player/BP_PlayerCamera.IsMove` true _camerapawn))
  (:`Released`
    (set `/Game/Blueprint/Player/BP_PlayerCamera.IsMove` false _camerapawn)))

(event `Key|X`
  (params (Key :type "Key Structure"))
  (:`Pressed`
    (if (`self.InputCharacter`)
      (`self.SendServer_DisableInputPawn`)
      (`KismetSystemLibrary.K2_ClearAndInvalidateTimerHandle` (`self.TimerCharacterInput`))
      (else
        (`self.SendServer_InputPawn` (`|GetArrayItem` (`self.CharacterSelects`)))
        (bind _returnvalue (`KismetSystemLibrary.K2_SetTimerDelegate` (delegate `CustomEvent_0`) (`GameplayStatics.GetWorldDeltaSeconds`) true))
        (set `self.TimerCharacterInput` _returnvalue)))))

(event `self.ReceiveBeginPlay`
  (`/Engine/EditorBlueprintResources/ActorMacros.Switch Has Authority`
    (:`Authority`
      (bind _returnvalue (`GameplayStatics.GetActorOfClass` "/Script/Engine.PlayerStart"))
      (bind _returnvalue_location (`KismetMathLibrary.BreakTransform` (`self.GetTransform` _returnvalue)))
      (bind _returnvalue_2 (`|SpawnActorFromClass` "/Game/Blueprint/Player/BP_PlayerCamera.BP_PlayerCamera_C" (`KismetMathLibrary.MakeTransform` _returnvalue_location) "Undefined" "OverrideRootScale" null self null))
      (bind _output_get (set `self.CameraPawn` _returnvalue_2))
      (`self.Possess` _output_get))))

(event `CustomEvent_0`
  (bind _pawninput (`self.PawnInput`))
  (if (`KismetMathLibrary.Vector_IsZero` (`self.GetVelocity` _pawninput))
    (`self.SetControlRotation` (`KismetMathLibrary.FindLookAtRotation` (`self.K2_GetActorLocation` _pawninput) (`.Location` (`GameplayStatics.BreakHitResult` (`self.GetHitResultUnderCursorByChannel` "TraceTypeQuery1")))))))

(event `InputAxis|CameraZoom`
  (params (AxisValue :type "Float (single-precision)"))
  (bind _camerapawn (`self.CameraPawn`))
  (`/Engine/EditorBlueprintResources/StandardMacros.IsValid` _camerapawn
    (:`Is Valid`
      (`CameraPlayerPawn.AddArmLenght` _camerapawn AxisValue 30.0))))

(event `InputAxis|MouseX`
  (params (AxisValue :type "Float (single-precision)"))
  (bind _camerapawn (`self.CameraPawn`))
  (`/Engine/EditorBlueprintResources/StandardMacros.IsValid` _camerapawn
    (:`Is Valid`
      (if (or (`/Game/Blueprint/Player/BP_PlayerCamera.IsRotatior` _camerapawn) (`/Game/Blueprint/Player/BP_PlayerCamera.IsMove` _camerapawn))
        (set `self.CameraYaw` (mod (+ (`self.CameraYaw`) (* AxisValue 5.0)) 360.0))))))

(event `InputAxis|MouseY`
  (params (AxisValue :type "Float (single-precision)"))
  (bind _camerapawn (`self.CameraPawn`))
  (`/Engine/EditorBlueprintResources/StandardMacros.IsValid` _camerapawn
    (:`Is Valid`
      (if (`/Game/Blueprint/Player/BP_PlayerCamera.IsMove` _camerapawn)
        (set `self.CameraPitch` (`KismetMathLibrary.FClamp` (+ (`self.CameraPitch`) (* AxisValue 5.0)) -80.0 -30.0))))))

(event `SendServer_InputPawn`
  (params (PawnInput :type "Pawn Object Reference"))
  (bind _pawninput (`self.PawnInput`))
  (bind _output_get (set `self.PawnInput` PawnInput))
  (set `self.AICharacter` (`AIBlueprintHelperLibrary.GetAIController` _output_get))
  (`self.Possess` _pawninput)
  (bind _ascharacter (cast `Character` _pawninput)
    (:`then`
      (`self.SendClients_EnableControllerYaw` _ascharacter true))
    (:`CastFailed`
      _))
  (set `self.InputCharacter` true)
  (`self.SetViewTargetWithBlend` (`self.CameraPawn`)))

(event `InputAxis|MoveForward`
  (params (AxisValue :type "Float (single-precision)"))
  (bind _pawninput (`self.PawnInput`))
  (`/Engine/EditorBlueprintResources/StandardMacros.IsValid` _pawninput
    (:`Is Valid`
      (bind _ascharacter (cast `Character` _pawninput)
        (:`then`
          (`Pawn.AddMovementInput` _ascharacter (`self.GetActorForwardVector` _pawninput) AxisValue false))
        (:`CastFailed`
          (bind _aswheeled_vehicle (cast `WheeledVehicle` _pawninput))
          (`WheeledVehicleMovementComponent.SetThrottleInput` (`WheeledVehicle.VehicleMovement` _aswheeled_vehicle) AxisValue))))))

(event `SendClients_EnableControllerYaw`
  (params (Target :type "Character Object Reference") (NewEnable :type Boolean))
  (if NewEnable
    (set `Pawn.bUseControllerRotationYaw` true Target)
    (set `CharacterMovementComponent.bOrientRotationToMovement` false (`Character.CharacterMovement` Target))
    (else
      (set `Pawn.bUseControllerRotationYaw` false Target)
      (set `CharacterMovementComponent.bOrientRotationToMovement` true (`Character.CharacterMovement` Target)))))

(event `InputAxis|MoveRight`
  (params (AxisValue :type "Float (single-precision)"))
  (bind _pawninput (`self.PawnInput`))
  (`/Engine/EditorBlueprintResources/StandardMacros.IsValid` _pawninput
    (:`Is Valid`
      (bind _ascharacter (cast `Character` _pawninput)
        (:`then`
          (`Pawn.AddMovementInput` _ascharacter (`self.GetActorRightVector` _pawninput) AxisValue false))
        (:`CastFailed`
          (bind _aswheeled_vehicle (cast `WheeledVehicle` _pawninput))
          (`WheeledVehicleMovementComponent.SetSteeringInput` (`WheeledVehicle.VehicleMovement` _aswheeled_vehicle) AxisValue))))))

(event `self.ReceiveTick`
  (params (DeltaSeconds :type "Float (single-precision)"))
  (bind _camerapawn (`self.CameraPawn`))
  (bind _camerapawn_2 (`self.CameraPawn`))
  (bind _springarm (`CameraPlayerPawn.SpringArm` _camerapawn))
  (bind _springarm_2 (`CameraPlayerPawn.SpringArm` _camerapawn_2))
  (if (not (`KismetSystemLibrary.IsDedicatedServer`))
    (`/Engine/EditorBlueprintResources/StandardMacros.IsValid` _camerapawn
      (:`Is Valid`
        (`SceneComponent.K2_SetRelativeRotation` _springarm (`KismetMathLibrary.RInterpTo` (`SceneComponent.RelativeRotation` _springarm) (`KismetMathLibrary.MakeRotator` (`self.CameraRoll`) (`self.CameraPitch`)) (`GameplayStatics.GetWorldDeltaSeconds`) 5.0) false false)
        (`self.K2_SetActorRotation` (`self.CameraPawn`) (`KismetMathLibrary.RInterpTo` (`self.K2_GetActorRotation` (`self.CameraPawn`)) (`KismetMathLibrary.MakeRotator` 0.0 0.0 (`self.CameraYaw`)) (`GameplayStatics.GetWorldDeltaSeconds`) 5.0) false)
        (set `SpringArmComponent.TargetArmLength` (`KismetMathLibrary.FInterpTo` (`SpringArmComponent.TargetArmLength` _springarm_2) (`CameraPlayerPawn.ArmLenght` _camerapawn_2) (`GameplayStatics.GetWorldDeltaSeconds`) 10.0) _springarm_2)))))

(fn `GetPawnCamera`
  (returns (ReturnValue :type "/Game/Blueprint/Player/BP_PlayerCamera Object Reference"))
  (bind _asbp_player_camera (cast `/Game/Blueprint/Player/BP_PlayerCamera` (`self.K2_GetPawn`)))
  (return _asbp_player_camera))

(fn `OnRep_CameraPawn`
  (set `CameraPlayerPawn.Player` self (`self.CameraPawn`)))

(fn `UserConstructionScript`)